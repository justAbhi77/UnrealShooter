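; Anim notify that plays a surface-specific landing sound for the shooter character when its jump-land animation reaches the notify.
; It casts the mesh owner to ShooterCharacterBP and queries its surface type to pick a metal, stone, tile, grass or water cue, defaulting to tile.
; The chosen cue plays at the owner's location, and owners that are not that character get no sound.
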(fn ReceivedNotify
  (params (MeshComp :type Skeletal%20Mesh%20Component%20Object%20Reference) (Animation :type Anim%20Sequence%20Base%20Object%20Reference) (EventReference :type Anim%20Notify%20Event%20Reference%20Structure%20%28by%20ref%29))
  (bind _returnvalue (Components|GetOwner MeshComp))
  (Utilities|FlowControl|Sequence
    (:then_0
      (bind _asshooter_character_bp (Utilities|Casting|CastToShooterCharacterBP _returnvalue))
      (bind _returnvalue_2 (Class|ShooterCharacter|GetSurfaceType _asshooter_character_bp))
      (Utilities|FlowControl|Sequence
        (:then_0
          (switch Utilities|FlowControl|Switch|SwitchonEPhysicalSurface _returnvalue_2
            (:SurfaceType_Default
              (LocalVariables|SetLandingSound "/Game/_Game/Assets/Sounds/Footsteps/Cue_Land_Tile.Cue_Land_Tile"))
            (:SurfaceType1
              (LocalVariables|SetLandingSound "/Game/_Game/Assets/Sounds/Footsteps/Cue_Land_Metal.Cue_Land_Metal"))
            (:SurfaceType2
              (LocalVariables|SetLandingSound "/Game/_Game/Assets/Sounds/Footsteps/Cue_Land_Stone.Cue_Land_Stone"))
            (:SurfaceType3
              (LocalVariables|SetLandingSound "/Game/_Game/Assets/Sounds/Footsteps/Cue_Land_Tile.Cue_Land_Tile"))
            (:SurfaceType4
              (LocalVariables|SetLandingSound "/Game/_Game/Assets/Sounds/Footsteps/Cue_Land_Grass.Cue_Land_Grass"))
            (:SurfaceType5
              (LocalVariables|SetLandingSound "/Game/_Game/Assets/Sounds/Footsteps/Cue_Land_Water.Cue_Land_Water"))))
        (:then_1
          (Audio|PlaySoundatLocation (LocalVariables|GetLandingSound) (Transformation|GetActorLocation _returnvalue) "0, 0, 0" 1.0 1.0 0.0 0 0 0 0))))
    (:then_1
      (return false))))