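; Footstep AnimNotify that plays a surface-specific sound and Niagara effect at a bone on the animated mesh.
; It casts the mesh owner to ShooterCharacterBP and switches on its surface type to pick both assets, defaulting to metal.
; Sound is gated by ShouldPlaySound, while particles spawn regardless.
; Each trigger also prints the bone and animation names for debugging.
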(fn ReceivedNotify
  (params (MeshComp :type Skeletal%20Mesh%20Component%20Object%20Reference) (Animation :type Anim%20Sequence%20Base%20Object%20Reference) (EventReference :type Anim%20Notify%20Event%20Reference%20Structure%20%28by%20ref%29))
  (Utilities|FlowControl|Sequence
    (:then_0
      (Development|PrintString (Utilities|String|Append (Utilities|String|ToString(Name) (Variables|Default|GetBoneName)) " " (Utilities|GetDisplayName Animation))))
    (:then_1
      (LocalVariables|SetLocalVar (Transformation|GetSocketLocation MeshComp (Variables|Default|GetBoneName)))
      (bind _asshooter_character_bp (Utilities|Casting|CastToShooterCharacterBP (Components|GetOwner MeshComp)))
      (bind _returnvalue (Class|ShooterCharacter|GetSurfaceType _asshooter_character_bp))
      (Utilities|FlowControl|Sequence
        (:then_0
          (switch Utilities|FlowControl|Switch|SwitchonEPhysicalSurface _returnvalue
            (:SurfaceType_Default
              (LocalVariables|SetFootstepSound "/Game/_Game/Assets/Sounds/Footsteps/Cue_Footstep_Metal.Cue_Footstep_Metal")
              (LocalVariables|SetNiagaraFootstepParticle "/Game/A_Surface_Footstep/Niagara_FX/ParticleSystems/PSN_General1_Surface.PSN_General1_Surface"))
            (:SurfaceType1
              (LocalVariables|SetFootstepSound "/Game/_Game/Assets/Sounds/Footsteps/Cue_Footstep_Metal.Cue_Footstep_Metal")
              (LocalVariables|SetNiagaraFootstepParticle "/Game/A_Surface_Footstep/Niagara_FX/ParticleSystems/PSN_General1_Surface.PSN_General1_Surface"))
            (:SurfaceType2
              (LocalVariables|SetFootstepSound "/Game/_Game/Assets/Sounds/Footsteps/Cue_Footstep_Stone.Cue_Footstep_Stone")
              (LocalVariables|SetNiagaraFootstepParticle "/Game/A_Surface_Footstep/Niagara_FX/ParticleSystems/PSN_Gravel_Surface.PSN_Gravel_Surface"))
            (:SurfaceType3
              (LocalVariables|SetFootstepSound "/Game/_Game/Assets/Sounds/Footsteps/Cue_Footstep_Tile.Cue_Footstep_Tile")
              (LocalVariables|SetNiagaraFootstepParticle "/Game/A_Surface_Footstep/Niagara_FX/ParticleSystems/PSN_General2_Surface.PSN_General2_Surface"))
            (:SurfaceType4
              (LocalVariables|SetFootstepSound "/Game/_Game/Assets/Sounds/Footsteps/Cue_Footstep_Grass.Cue_Footstep_Grass")
              (LocalVariables|SetNiagaraFootstepParticle "/Game/A_Surface_Footstep/Niagara_FX/ParticleSystems/PSN_Grass_Surface.PSN_Grass_Surface"))
            (:SurfaceType5
              (LocalVariables|SetFootstepSound "/Game/_Game/Assets/Sounds/Footsteps/Cue_Footstep_Water.Cue_Footstep_Water")
              (LocalVariables|SetNiagaraFootstepParticle "/Game/A_Surface_Footstep/Niagara_FX/ParticleSystems/PSN_WaterLight_Surface.PSN_WaterLight_Surface"))))
        (:then_1
          (if (Variables|Default|GetbShouldPlaySound)
            (Audio|PlaySoundatLocation (LocalVariables|GetFootstepSound) (LocalVariables|GetLocalVar) "0, 0, 0" 1.0 1.0 0.0 0 0 0 0))
          (Niagara|SpawnSystematLocation (LocalVariables|GetNiagaraFootstepParticle) (LocalVariables|GetLocalVar)))))
    (:then_2
      (return true))))