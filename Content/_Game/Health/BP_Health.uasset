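; BP_Health is a health pickup that heals the shooter character on overlap.
; When a ShooterCharacterBP enters the Sphere, a DoOnce adds HealingAmount to its Health, clamped between zero and MaxHealth.
; The pickup then plays a sound at its location and destroys itself.
; Tick does nothing, as the yaw spin logic for the SMHealth component is disconnected and never runs.
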(event OnComponentBeginOverlap(Sphere)
  (params (OverlappedComponent :type Primitive%20Component%20Object%20Reference) (OtherActor :type Actor%20Object%20Reference) (OtherComp :type Primitive%20Component%20Object%20Reference) (OtherBodyIndex :type Integer) (bFromSweep :type Boolean) (SweepResult :type Hit%20Result%20Structure%20%28by%20ref%29))
  ;[1 1 1] Overlap
  (bind _asshooter_character_bp (Utilities|Casting|CastToShooterCharacterBP OtherActor))
  (Utilities|FlowControl|DoOnce false
    (:Completed
      (Variables|/Script/Shooter.ShooterCharacter|SetHealth _asshooter_character_bp (Math|Float|Clamp(Float) (+ (Variables|/Script/Shooter.ShooterCharacter|GetHealth _asshooter_character_bp) (Variables|Default|GetHealingAmount)) 0.0 (Variables|/Script/Shooter.ShooterCharacter|GetMaxHealth _asshooter_character_bp)))
      (Audio|PlaySoundatLocation (Variables|Default|GetHealthPickupSound) (Transformation|GetActorLocation) "0, 0, 0" 1.0 1.0 0.0 0 0 0 0)
      (Actor|DestroyActor))))

(event EventTick
  (params (DeltaSeconds :type Float%20%28single-precision%29))
  ;[1 1 1] (Custom-Tick) Animation
)

(fn ConstructionScript)