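; Shooter HUD that draws a dynamic crosshair near screen center, raised slightly above it.
; BeginPlay caches the player's ShooterCharacterBP after a short delay, and DrawHUD re-fetches it whenever the reference is invalid.
; Each frame it draws five textures from the equipped weapon, pushing top, bottom, left and right outward by the character's spread multiplier times a maximum spread.
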(event EventBeginPlay
  ;[1 1 1] Cache Player
  (Utilities|IsValid (Variables|Private|GetShooterCharacter)
    (:Is%20Not%20Valid
      (Utilities|FlowControl|Delay 0.2)
      (bind _asshooter_character_bp (Utilities|Casting|CastToShooterCharacterBP (Game|Player|GetPlayerPawn 0)))
      (Variables|Private|SetShooterCharacter _asshooter_character_bp))))

(event EventDrawHUD
  (params (SizeX :type Integer) (SizeY :type Integer))
  (bind _output_get (Variables|Private|SetScreenCenter (Math|Vector2D|MakeVector2D (Math|Conversions|ToFloat(Integer) (/ SizeX 2)) (Math|Conversions|ToFloat(Integer) (/ SizeY 2)))))
  (Variables|Private|SetCrosshairBaseCenter (Math|Vector2D|MakeVector2D (- (.x _output_get) (Variables|Private|GetCrosshairHalfWidth)) (Utilities|Operators|Subtract (.y _output_get) (Variables|Private|GetCrosshairHalfHeight) 5e+01)))
  (Variables|Private|GetShooterCharacter
    (:then
      _)
    (:else
      (bind _asshooter_character_bp (Utilities|Casting|CastToShooterCharacterBP (Game|Player|GetPlayerPawn 0)))
      (Variables|Private|SetShooterCharacter _asshooter_character_bp)))
  (Variables|Private|SetCrosshairSpreadMultiplier (Class|ShooterCharacter|GetCrosshairSpreadMultiplier (Variables|Private|GetShooterCharacter)))
  (Canvas|DrawTexture (Variables|/Script/Shooter.Weapon|GetCrosshairsBottom (Variables|/Script/Shooter.ShooterCharacter|GetEquippedWeapon (Variables|Private|GetShooterCharacter))) (.x (Variables|Private|GetCrosshairBaseCenter)) (+ (.y (Variables|Private|GetCrosshairBaseCenter)) (* (Variables|Private|GetCrosshairSpreadMax) (Variables|Private|GetCrosshairSpreadMultiplier))) 64.0 64.0 0.0 0.0 1.0 1.0 "(R=1.000000,G=1.000000,B=1.000000,A=1.000000)")
  (Canvas|DrawTexture (Variables|/Script/Shooter.Weapon|GetCrosshairsTop (Variables|/Script/Shooter.ShooterCharacter|GetEquippedWeapon (Variables|Private|GetShooterCharacter))) (.x (Variables|Private|GetCrosshairBaseCenter)) (- (.y (Variables|Private|GetCrosshairBaseCenter)) (* (Variables|Private|GetCrosshairSpreadMax) (Variables|Private|GetCrosshairSpreadMultiplier))) 64.0 64.0 0.0 0.0 1.0 1.0 "(R=1.000000,G=1.000000,B=1.000000,A=1.000000)")
  (Canvas|DrawTexture (Variables|/Script/Shooter.Weapon|GetCrosshairsLeft (Variables|/Script/Shooter.ShooterCharacter|GetEquippedWeapon (Variables|Private|GetShooterCharacter))) (- (.x (Variables|Private|GetCrosshairBaseCenter)) (* (Variables|Private|GetCrosshairSpreadMax) (Variables|Private|GetCrosshairSpreadMultiplier))) (.y (Variables|Private|GetCrosshairBaseCenter)) 64.0 64.0 0.0 0.0 1.0 1.0 "(R=1.000000,G=1.000000,B=1.000000,A=1.000000)")
  (Canvas|DrawTexture (Variables|/Script/Shooter.Weapon|GetCrosshairsRight (Variables|/Script/Shooter.ShooterCharacter|GetEquippedWeapon (Variables|Private|GetShooterCharacter))) (+ (.x (Variables|Private|GetCrosshairBaseCenter)) (* (Variables|Private|GetCrosshairSpreadMax) (Variables|Private|GetCrosshairSpreadMultiplier))) (.y (Variables|Private|GetCrosshairBaseCenter)) 64.0 64.0 0.0 0.0 1.0 1.0 "(R=1.000000,G=1.000000,B=1.000000,A=1.000000)")
  (Canvas|DrawTexture (Variables|/Script/Shooter.Weapon|GetCrosshairsMiddle (Variables|/Script/Shooter.ShooterCharacter|GetEquippedWeapon (Variables|Private|GetShooterCharacter))) (.x (Variables|Private|GetCrosshairBaseCenter)) (.y (Variables|Private|GetCrosshairBaseCenter)) 64.0 64.0 0.0 0.0 1.0 1.0 "(R=1.000000,G=1.000000,B=1.000000,A=1.000000)"))

(fn ConstructionScript)